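; Player-side shop component that handles item pricing, selling and per-item sale records.
; Input actions adjust the selling price shown in the selling interface widget and, when in a shop with a free display, place the inventory item there at that price.
; Saved sales keep the highest price per item and outcome (fail, sell, cheap), then refresh the registered stat panels.
; Tick pushes the in-shop state to the widget.
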(event Custom|Event_RestPrice
  ;[0 1 0.1575] Reset Price
  (bind _output_get (Variables|Default|SetSellingPrice 0.0))
  (Default|EventUpdatePrice (Variables|Default|GetInterface_Ref) _output_get))

(event Custom|Event_Addpannel
  (params (PannelRef :type Bp%20Sells%20Pannel%20Object%20Reference) (ItemId :type Integer))
  ;[1 1 1] Get the pannel Ref
  (Utilities|Array|SetArrayElem (Variables|Default|GetSellStatsPannel) ItemId PannelRef))

(event Custom|Event_SaveStats
  (params (Item_ID :type Integer) (TypeOfSell :type Integer) (Price :type Float%20%28double-precision%29))
  ;[0.193 0.5251 0.5469] Sell Stat Saving
  (Development|PrintText (Utilities|Text|FormatText "Try save sats  
id : {id}  
type : {type}  
Price : {Price} " Item_ID TypeOfSell Price) true true "(R=1.000000,G=0.070607,B=0.000000,A=1.000000)" 1e+01)
  (Variables|Default|SetStats_TypeOfSell_Portal TypeOfSell)
  (Variables|Default|SetStats_ItemId_Portal Item_ID)
  (Variables|Default|SetStats_Price_Portal Price)
  (switch int (Variables|Default|GetStats_ItemId_Portal)
    (:0
      (bind _return (CallFunction|PriceCheck (Variables|Default|GetOrange_0_Stats)))
      (if _return
        (Utilities|Array|SetArrayElem (Variables|Default|GetOrange_0_Stats) (Variables|Default|GetStats_TypeOfSell_Portal) (Variables|Default|GetStats_Price_Portal))
        (Default|CallSellPannelDisplay :!label _label)
        (Development|PrintString "Try update display")))
    (:1
      (bind _return_2 (CallFunction|PriceCheck (Variables|Default|GetBlue_1_Stats)))
      (if _return_2
        (Utilities|Array|SetArrayElem (Variables|Default|GetBlue_1_Stats) (Variables|Default|GetStats_TypeOfSell_Portal) (Variables|Default|GetStats_Price_Portal))
        (goto _label)))
    (:2
      (bind _return_3 (CallFunction|PriceCheck (Variables|Default|GetPurple_2_stats)))
      (if _return_3
        (Utilities|Array|SetArrayElem (Variables|Default|GetPurple_2_stats) (Variables|Default|GetStats_TypeOfSell_Portal) (Variables|Default|GetStats_Price_Portal))
        (goto _label)))
    (:3
      (bind _return_4 (CallFunction|PriceCheck (Variables|Default|GetGreen_3_Stats)))
      (if _return_4
        (Utilities|Array|SetArrayElem (Variables|Default|GetGreen_3_Stats) (Variables|Default|GetStats_TypeOfSell_Portal) (Variables|Default|GetStats_Price_Portal))
        (goto _label)))))

(event Input|EnhancedActionEvents|EnhancedInputActionIA_Sell
  (params (ActionValue :type Boolean) (ElapsedSeconds :type Float%20%28double-precision%29) (TriggeredSeconds :type Float%20%28double-precision%29) (InputAction :type Input%20Action%20Object%20Reference :default "/Game/TopDown/Input/Actions/IA_Sell.IA_Sell"))
  ;[0.06771 0.06771 0.06771] INPUT
  (:Started
    (if (and (Variables|Default|GetIs%20in%20Shop) (Variables|/Game/Shop/Blueprint/BP_Selling_Display.BP_Selling_Display_C|GetIsFree (Variables|/Game/Shop/Blueprint/BP_Selling_Point.BP_Selling_Point_C|GetDIsplay_Ref (Variables|Default|GetShop_Ref))))
      (Default|EventAddItem (Variables|/Game/Shop/Blueprint/BP_Selling_Point.BP_Selling_Point_C|GetDIsplay_Ref (Variables|Default|GetShop_Ref)) (Variables|Default|GetInventory) (Variables|Default|GetSellingPrice)))))

(event Input|EnhancedActionEvents|EnhancedInputActionIA_PriceIncrease
  (params (ActionValue :type Boolean) (ElapsedSeconds :type Float%20%28double-precision%29) (TriggeredSeconds :type Float%20%28double-precision%29) (InputAction :type Input%20Action%20Object%20Reference :default "/Game/TopDown/Input/Actions/IA_PriceIncrease.IA_PriceIncrease"))
  ;[0.06771 0.06771 0.06771] INPUT
  (bind _output_get (Variables|Default|SetSellingPrice (+ (Variables|Default|GetSellingPrice) 1.0)))
  (Default|EventUpdatePrice (Variables|Default|GetInterface_Ref) _output_get))

(event Input|EnhancedActionEvents|EnhancedInputActionIA_PriceDeacrease
  (params (ActionValue :type Boolean) (ElapsedSeconds :type Float%20%28double-precision%29) (TriggeredSeconds :type Float%20%28double-precision%29) (InputAction :type Input%20Action%20Object%20Reference :default "/Game/TopDown/Input/Actions/IA_PriceDeacrease.IA_PriceDeacrease"))
  ;[0.06771 0.06771 0.06771] INPUT
  (if (> (Variables|Default|GetSellingPrice) 0.0)
    (bind _output_get (Variables|Default|SetSellingPrice (- (Variables|Default|GetSellingPrice) 1.0)))
    (Default|EventUpdatePrice (Variables|Default|GetInterface_Ref) _output_get)))

(event EventTick
  (params (DeltaSeconds :type Float%20%28single-precision%29))
  ;[1 0 0] Event tick
  (Default|EventDispayPrice (Variables|Default|GetInterface_Ref) (Variables|Default|GetIs%20in%20Shop)))

(event EventBeginPlay
  ;[1 0 0] Begin play
  ;;[1 1 1] Ui Set
  (bind _returnvalue (UserInterface|CreateWidget "/Game/Shop/Ui/WB_SellingInterface.WB_SellingInterface_C"))
  (Variables|Default|SetInterface_Ref _returnvalue)
  (UserInterface|Viewport|AddtoViewport (Variables|Default|GetInterface_Ref) 0)
  (bind _output_get (Variables|Default|SetSellingPrice 0.0))
  (Default|EventUpdatePrice (Variables|Default|GetInterface_Ref) _output_get)
  (Default|CallAddPannel))

(fn PriceCheck
  (params (StatsArray :type Array%20of%20Floats%20%28double-precision%29))
  (bind _stats_price_portal (Variables|Default|GetStats_Price_Portal))
  (bind _stats_typeofsell_portal (Variables|Default|GetStats_TypeOfSell_Portal))
  (bind _output (Utilities|Array|Get(acopy) StatsArray _stats_typeofsell_portal))
  (Development|PrintText (Utilities|Text|FormatText "Try Price check  
sell type : {type}  
old : {old}  
new : {new} " (Variables|Default|GetStats_TypeOfSell_Portal) _output _stats_price_portal) true true "(R=1.000000,G=0.000000,B=0.070318,A=1.000000)" 1e+01)
  (return (< _output _stats_price_portal)))

(fn FunctionSendSellStatistic
  (params (ItemId :type Integer))
  (bind _orange_0_stats (Variables|Default|GetOrange_0_Stats))
  (bind _blue_1_stats (Variables|Default|GetBlue_1_Stats))
  (bind _purple_2_stats (Variables|Default|GetPurple_2_stats))
  (bind _green_3_stats (Variables|Default|GetGreen_3_Stats))
  (switch int ItemId
    (:0
      (return (Utilities|Array|Get(acopy) _orange_0_stats) (Utilities|Array|Get(acopy) _orange_0_stats 1) (Utilities|Array|Get(acopy) _orange_0_stats 2)))
    (:1
      (return (Utilities|Array|Get(acopy) _blue_1_stats) (Utilities|Array|Get(acopy) _blue_1_stats 1) (Utilities|Array|Get(acopy) _blue_1_stats 2)))
    (:2
      (return (Utilities|Array|Get(acopy) _purple_2_stats) (Utilities|Array|Get(acopy) _purple_2_stats 1) (Utilities|Array|Get(acopy) _purple_2_stats 2)))
    (:3
      (return (Utilities|Array|Get(acopy) _green_3_stats) (Utilities|Array|Get(acopy) _green_3_stats 1) (Utilities|Array|Get(acopy) _green_3_stats 2)))))