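; BP_SellTimer is a shop countdown that periodically signals when the next sell happens.
; A looping one-second timer started on BeginPlay decrements the remaining time, then resets it and fires CallToSell once it has run out.
; Each tick of that timer also writes the remaining time to the Display text.
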(event Custom|Event_SellTimer
  (if (> (Variables|Default|GetTimer) 0.0)
    (Variables|Default|SetTimer (- (Variables|Default|GetTimer) 1.0))
    (else
      (Variables|Default|SetTimer 1e+01)
      (Default|CallCalltoSell)))
  (Rendering|Components|TextRender|SetText (Variables|Default|Getdisplay) (Utilities|Text|FormatText "Time before the next sell : {time}" (Variables|Default|GetTimer))))

(event EventBeginPlay
  (Utilities|Time|SetTimerbyEvent (delegate Custom|Event_SellTimer) 1.0 true))

(fn ConstructionScript)