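; Shop display slot that shows one priced item for sale and judges its price when the sale timer fires.
; Adding an item spawns a cube mesh at the placeholder's transform, with material and name looked up by ID in DT_Selling_Item.
; Timer dispatchers trigger selling, which lights an expensive, perfect or gifted light against the item's price range and saves the result to the player's BPCShop, or reset, which clears the slot.
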(event Custom|Event_AddItem
  (params (Item_ID :type Integer) (Price :type Float%20%28double-precision%29))
  ;[1 1 1] AddItem
  (Variables|Default|SetItem%20ID Item_ID)
  (Variables|Default|SetPrice Price)
  (bind _returnvalue (AddComponent|AddStaticMeshComponent false (Variables|Default|GetItem_Transform)))
  (Variables|Default|SetItemRef _returnvalue)
  (Components|StaticMesh|SetStaticMesh (Variables|Default|GetItemRef) "/Game/Shop/Props/SM_Cube_01.SM_Cube_01")
  (Variables|Default|SetIsFree false)
  (bind (_itemname _itemprice _itemmaterial) (CallFunction|FunctionGetData))
  (Rendering|Material|SetMaterial (Variables|Default|GetItemRef) 0 _itemmaterial)
  (Rendering|Components|TextRender|SetText (Variables|Default|GetTextName) (Utilities|Text|ToText(String) _itemname))
  (Rendering|Components|TextRender|SetText (Variables|Default|GetTextPrice) (Utilities|Text|ToText(Float) (Variables|Default|GetPrice) "HalfToEven")))

(event Custom|Event_Reset
  ;[1 1 1] ResetShop
  (Components|DestroyComponent (Variables|Default|GetItemRef))
  (Variables|Default|SetIsFree true)
  (Rendering|Components|Light|SetIntensity (Variables|Default|GetLight_Expencive) 0.0))

(event Custom|CallSell
  ;[1 0 0] BeginPlay
  ;;[1 0.4155 0] Selling Dispatcher
  (CallFunction|EventSelling))

(event Custom|Event_Selling
  ;[0.4531 0.3519 0.09909] Selling Event
  (if (not (Variables|Default|GetIsFree))
    (bind _itemprice (CallFunction|FunctionGetData))
    ;;[1 1 1] Price is to Hight
    (if (> (Variables|Default|GetPrice) (.y _itemprice))
      (Rendering|Components|Light|SetIntensity (Variables|Default|GetLight_Expencive) 5e+03)
      (Default|EventSaveStats (Variables|Default|GetRef_BPCShop) (Variables|Default|GetItem%20ID) 0 (Variables|Default|GetPrice))
      (else
        ;;[1 1 1] Price Too Low
        (if (< (Variables|Default|GetPrice) (.x _itemprice))
          (Rendering|Components|Light|SetIntensity (Variables|Default|GetLight_Gifted) 5e+03)
          (Default|EventSaveStats (Variables|Default|GetRef_BPCShop) (Variables|Default|GetItem%20ID) 2 (Variables|Default|GetPrice))
          (else
            ;;[1 1 1] Price Ok
            (Rendering|Components|Light|SetIntensity (Variables|Default|GetLight_Perfect) 5e+03)
            (Default|EventSaveStats (Variables|Default|GetRef_BPCShop) (Variables|Default|GetItem%20ID) 1 (Variables|Default|GetPrice))))))))

(event Custom|CallReset
  ;[1 0 0] BeginPlay
  ;;[1 0.4155 0] Selling Dispatcher
  (CallFunction|EventReset))

(event EventBeginPlay
  ;[1 0 0] BeginPlay
  (CallFunction|EventReset)
  (Variables|Default|SetRef_BPCShop (Variables|/Game/TopDown/Blueprints/BP_TopDownCharacter.BP_TopDownCharacter_C|GetBPC_Shop (.AsBP%20Top%20Down%20Character (Utilities|Casting|CastToBP_TopDownCharacter (Game|GetPlayerCharacter 0)))))
  ;;[1 0.4155 0] Selling Dispatcher
  (EventDispatchers|BindEventtoCalltoSell (Variables|Default|GetRef_Timer) (delegate Custom|CallSell))
  (EventDispatchers|BindEventtoCallReset (Variables|Default|GetRef_Timer) (delegate Custom|CallReset)))

(fn ConstructionScript
  (Variables|Default|SetItem_Transform (Transformation|GetRelativeTransform (Variables|Default|GetStaticMesh))))

(fn FunctionGetData
  (bind _outrownames (DataTable|GetDataTableRowNames "/Game/Shop/Data/DT_Selling_Item.DT_Selling_Item"))
  (bind _array_element (Utilities|Array|ForEachLoopwithBreak _outrownames)
    (:LoopBody
      (bind _returnvalue (Utilities|GetDataTableRow "/Game/Shop/Data/DT_Selling_Item.DT_Selling_Item" _array_element)
        (:then
          (if (== (.id _returnvalue) (Variables|Default|GetItem%20ID))
            (return (.name _returnvalue) (.prix_ok _returnvalue) (.material _returnvalue))))))))