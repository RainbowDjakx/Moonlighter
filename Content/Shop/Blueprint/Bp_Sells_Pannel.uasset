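; Shop panel actor that displays sale price statistics for one ItemID: max expensive, max good sell and min cheap.
; On BeginPlay it binds to the player character's BPCShop component's panel display event.
; When that fires, it queries the component's sell statistics and writes the formatted dollar values to three texts.
; An uncalled data table lookup on DT_Selling_Item is a stub that iterates column names and returns zeros.
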(event Custom|Event_EditLow
  (params (Input :type Float%20%28double-precision%29))
  ;[1 1 1] Update Vallue
  (Rendering|Components|TextRender|SetText (Variables|Default|Getlow) (Utilities|Text|FormatText "Min Cheap : {vallue} $ " Input)))

(event Custom|Event_EditHight
  (params (Input :type Float%20%28double-precision%29))
  ;[1 1 1] Update Vallue
  (Rendering|Components|TextRender|SetText (Variables|Default|Getmax) (Utilities|Text|FormatText "Max Expencive : {vallue} $ " Input)))

(event Custom|Event_PannelDisplay
  ;[1 0 0] Pannel Setup
  (bind (_hightest_fail _highest_sell _highest_cheap) (Default|FunctionSendSellStatistic (Variables|/Game/TopDown/Blueprints/BP_TopDownCharacter.BP_TopDownCharacter_C|GetBPC_Shop (.AsBP%20Top%20Down%20Character (Utilities|Casting|CastToBP_TopDownCharacter (Game|GetPlayerCharacter 0)))) (Variables|Default|GetItemID)))
  (CallFunction|EventUpdateAll _hightest_fail _highest_sell _highest_cheap)
  (Development|PrintString "Update price"))

(event Custom|Event_EditGood
  (params (Input :type Float%20%28double-precision%29))
  ;[1 1 1] Update Vallue
  (Rendering|Components|TextRender|SetText (Variables|Default|GetGood) (Utilities|Text|FormatText "Max Good sell : {vallue} $ " Input)))

(event Custom|Event_UpdateAll
  (params (Hight :type Float%20%28double-precision%29) (Ok :type Float%20%28double-precision%29) (Low :type Float%20%28double-precision%29))
  ;[1 1 1] Update Vallue
  (CallFunction|EventEditHight Hight)
  (CallFunction|EventEditGood Ok)
  (CallFunction|EventEditLow Low))

(event EventBeginPlay
  ;[1 0 0] Pannel Setup
  (EventDispatchers|BindEventtoSellPannelDisplay (Variables|/Game/TopDown/Blueprints/BP_TopDownCharacter.BP_TopDownCharacter_C|GetBPC_Shop (.AsBP%20Top%20Down%20Character (Utilities|Casting|CastToBP_TopDownCharacter (Game|GetPlayerCharacter 0)))) (delegate Custom|Event_PannelDisplay)))

(fn ConstructionScript)

(fn FuctionGetData
  (params (ItemID :type Integer))
  (bind _outcolumnnames (Class|DataTableFunctionLibrary|GetDataTableColumnNames "/Game/Shop/Data/DT_Selling_Item.DT_Selling_Item"))
  (bind _array_element (Utilities|Array|ForEachLoopwithBreak _outcolumnnames)
    (:LoopBody
      (bind _returnvalue (Utilities|GetDataTableRow "/Game/Shop/Data/DT_Selling_Item.DT_Selling_Item" _array_element)
        (:then
          (if (== (.id _returnvalue) ItemID)
            (return 0.0 0.0 0.0)))))))