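; BP_ItemSelecteur is a shop prop: a spinning cube whose material reflects its item type.
; The construction script switches on ItemType to assign one of four cube material instances to SMCube01.
; Tick adds a fixed yaw step to the cube's world rotation each frame without using delta time, so spin speed depends on frame rate.
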(event EventBeginPlay)

(event Collision|EventActorBeginOverlap
  (params (OtherActor :type Actor%20Object%20Reference)))

(event EventTick
  (params (DeltaSeconds :type Float%20%28single-precision%29))
  (bind _sm_cube_01 (Variables|Default|GetSM_Cube_01))
  (bind _returnvalue (Transformation|GetWorldRotation _sm_cube_01))
  (Transformation|SetWorldRotation (Variables|Default|GetSM_Cube_01) (Math|Rotator|MakeRotator (.roll _returnvalue) (.pitch _returnvalue) (+ (.yaw _returnvalue) 1.0)) false false))

(fn ConstructionScript
  ;[1 1 1] Couleur En fonction Du type d'item
  (switch int (Variables|Default|GetItemType)
    (:0
      (Rendering|Material|SetMaterial (Variables|Default|GetSM_Cube_01) 0 "/Game/Shop/Material/MI_Cube_01.MI_Cube_01"))
    (:1
      (Rendering|Material|SetMaterial (Variables|Default|GetSM_Cube_01) 0 "/Game/Shop/Material/MI_Cube_02.MI_Cube_02"))
    (:2
      (Rendering|Material|SetMaterial (Variables|Default|GetSM_Cube_01) 0 "/Game/Shop/Material/MI_Cube_03.MI_Cube_03"))
    (:3
      (Rendering|Material|SetMaterial (Variables|Default|GetSM_Cube_01) 0 "/Game/Shop/Material/MI_Cube_04.MI_Cube_04"))))